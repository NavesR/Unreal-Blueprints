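; BP_Door_3 is a sliding door that the player opens and closes with E while standing in its trigger box.
; Box overlap with the FirstPersonCharacter toggles input; leaving also reverses the slide after a one-second delay.
; A FlipFlop plays or reverses the DoorSlide timeline, moving InnerDoorPiece along local Z.
; IsDoorLocked works inverted: true permits opening and makes Tick show "UNLOCKED", false shows "LOCKED".
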(event `self.ReceiveTick`
  (params (DeltaSeconds :type "Float (single-precision)"))
  (bind _lockedtext (`self.LockedText`))
  (if (`self.IsDoorLocked`)
    (`TextRenderComponent.K2_SetText` _lockedtext "UNLOCKED")
    (else
      (`TextRenderComponent.K2_SetText` _lockedtext "LOCKED"))))

(event `self.BoxTrigger.OnComponentBeginOverlap`
  (params (OverlappedComponent :type "PrimitiveComponent Object Reference") (OtherActor :type "Actor Object Reference") (OtherComp :type "PrimitiveComponent Object Reference") (OtherBodyIndex :type Integer) (bFromSweep :type Boolean) (SweepResult :type "HitResult Structure (by ref)"))
  ;[1 1 1] DOOR
  (cast `/Game/FirstPersonBP/Blueprints/FirstPersonCharacter` OtherActor)
  (`self.EnableInput` (`GameplayStatics.GetPlayerController` 0)))

(event `Key|E`
  (params (Key :type "Key Structure"))
  ;[1 1 1] DOOR
  (:`Pressed`
    (if (`self.IsDoorLocked`)
      (`/Engine/EditorBlueprintResources/StandardMacros.FlipFlop`
        (:`A`
          (bind (_direction _slideamaunt) (`Timeline|DoorSlide` :!label _label)
            (:`Update`
              (`SceneComponent.K2_SetRelativeLocation` (`self.InnerDoorPiece`) (`KismetMathLibrary.MakeVector` 0.0 0.0 (* _slideamaunt 49.0)) false false))))
        (:`B`
          (goto _label :!via `Reverse`))))))

(event `self.BoxTrigger.OnComponentEndOverlap`
  (params (OverlappedComponent :type "PrimitiveComponent Object Reference") (OtherActor :type "Actor Object Reference") (OtherComp :type "PrimitiveComponent Object Reference") (OtherBodyIndex :type Integer))
  ;[1 1 1] DOOR
  (cast `/Game/FirstPersonBP/Blueprints/FirstPersonCharacter` OtherActor)
  (`self.DisableInput` (`GameplayStatics.GetPlayerController` 0))
  (`KismetSystemLibrary.Delay` 1.0)
  (goto _label :!via `Reverse`))

(fn `UserConstructionScript`)